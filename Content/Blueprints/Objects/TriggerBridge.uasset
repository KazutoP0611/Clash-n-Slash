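; A bridge actor that advances in stages from a start point to an end point as its linked triggers fire.
; BeginPlay binds the triggers' GotTriggered event and divides the travel distance by the trigger count.
; Each trigger sets the next target, optionally plays a level sequence between delays, then starts movement.
; Tick moves the bridge at constant speed over a set duration, disabling the Box collision after the final stage.
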(event `self.ReceiveBeginPlay`
  ;[1 1 1] Set Up Call Event
  (if (`KismetArrayLibrary.Array_IsValidIndex` (`self.ArrayOfTrigger`))
    (add `/Game/Blueprints/Objects/TriggerFireLight_BP.GotTriggered` (`self.ArrayOfTrigger`) (delegate `CheckTriggered`)))
  (`SceneComponent.K2_SetRelativeLocation` (`self.Moving Bridge`) (`self.StartPoint`) false false)
  (set `self.VectorPerRound` (/ (- (`self.EndPoint`) (`self.StartPoint`)) (`KismetArrayLibrary.Array_Length` (`self.ArrayOfTrigger`)))))

(event `Play Squence`
  (bind _levelsequence (`self.LevelSequence`))
  ;[1 1 1] Play Sequence
  (`/Engine/EditorBlueprintResources/StandardMacros.IsValid` _levelsequence
    (:`Is Valid`
      (bind _outactor (`LevelSequencePlayer.CreateLevelSequencePlayer` _levelsequence))
      (`MovieSceneSequencePlayer.Play` (`LevelSequenceActor.SequencePlayer` _outactor)))))

(event `CheckTriggered`
  ;[1 1 1] Set Up Call Event
  (set `self.TriggeredCount` (+ 1 (`self.TriggeredCount`)))
  (if (== (`self.TriggeredCount`) (`KismetArrayLibrary.Array_Length` (`self.ArrayOfTrigger`)))
    (set `self.ShouldMoveThisRound` (`self.EndPoint`))
    (else
      (set `self.ShouldMoveThisRound` (+ (`self.VectorPerRound`) (`SceneComponent.RelativeLocation` (`self.Moving Bridge`))))))
  (set `self.ThisRoundStartPoint` (`SceneComponent.RelativeLocation` (`self.Moving Bridge`)))
  (`/Engine/EditorBlueprintResources/StandardMacros.IsValid` (`self.LevelSequence`)
    (:`Is Valid`
      (`KismetSystemLibrary.Delay` (`self.DelayBeforePlaySequence`))
      (`self.Play Squence`)
      (`KismetSystemLibrary.Delay` (`self.DelayAfterPlaySequence`)))
    (:`Is Not Valid`
      _))
  (`self.MoveGate`))

(event `MoveGate`
  ;[1 1 1] Move the gate
  (set `self.ShouldMove` true))

(event `self.ReceiveTick`
  (params (DeltaSeconds :type "Float (single-precision)"))
  ;[1 1 1] Move the gate
  (if (`self.ShouldMove`)
    (`SceneComponent.K2_SetRelativeLocation` (`self.Moving Bridge`) (`KismetMathLibrary.VInterpTo_Constant` (`SceneComponent.RelativeLocation` (`self.Moving Bridge`)) (`self.ShouldMoveThisRound`) DeltaSeconds (/ (`KismetMathLibrary.Vector_Distance` (`self.ThisRoundStartPoint`) (`self.ShouldMoveThisRound`)) (`self.MoveInSeconds`))) false false)
    (if (== (`SceneComponent.RelativeLocation` (`self.Moving Bridge`)) (`self.ShouldMoveThisRound`) :`ErrorTolerance` 0.01)
      (set `self.ShouldMove` false)
      (if (== (`self.TriggeredCount`) (`KismetArrayLibrary.Array_Length` (`self.ArrayOfTrigger`)))
        (`PrimitiveComponent.SetCollisionEnabled` (`self.Box`) "NoCollision")))))

(fn `UserConstructionScript`)