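; Boss arena trigger box that starts the boss intro the first time the ThirdPersonCharacter overlaps its collision component.
; An IsTriggered flag makes it one-shot, and configurable delays pace the cutscene and the boss activation that follows.
; The cutscene plays an optional Level Sequence through a player created at runtime.
; Activation makes the referenced EnemyBoss's fire visible, then enables its boss sense after short fixed delays.
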(event `self.CollisionComponent.OnComponentBeginOverlap`
  (params (OverlappedComponent :type "PrimitiveComponent Object Reference") (OtherActor :type "Actor Object Reference") (OtherComp :type "PrimitiveComponent Object Reference") (OtherBodyIndex :type Integer) (bFromSweep :type Boolean) (SweepResult :type "HitResult Structure (by ref)"))
  ;[1 1 1] Overlap Event
  (cast `/Game/ThirdPersonBP/Blueprints/ThirdPersonCharacter` OtherActor)
  (if (not (`self.isTriggered`))
    (set `self.isTriggered` true)
    (`KismetSystemLibrary.Delay` (`self.DelayBeforePlaySequence`))
    (`self.PlayCutScene`)
    (`KismetSystemLibrary.Delay` (`self.DelayAfterPlaySequence`))
    (`self.Activate Boss`)))

(event `PlayCutScene`
  (bind _levelsequence (`self.LevelSequence`))
  ;[1 1 1] Play Sequence
  (`/Engine/EditorBlueprintResources/StandardMacros.IsValid` _levelsequence
    (:`Is Valid`
      (bind _outactor (`LevelSequencePlayer.CreateLevelSequencePlayer` _levelsequence))
      (`MovieSceneSequencePlayer.Play` (`LevelSequenceActor.SequencePlayer` _outactor)))))

(event `Activate Boss`
  (bind _enemy_boss (`self.Enemy Boss`))
  ;[1 1 1] Activate Boss
  (`KismetSystemLibrary.Delay` 0.2)
  (`/Game/Blueprints/Enemies/CNS_Enemy_Bose_BP.Set Fire Visibility` _enemy_boss true)
  (`KismetSystemLibrary.Delay` 2.0)
  (`/Game/Blueprints/Enemies/CNS_Enemy_Bose_BP.Activate Boss Sense` _enemy_boss))

(fn `UserConstructionScript`)