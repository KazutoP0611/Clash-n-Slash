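; BossGate is a gate actor that opens once the referenced boss dies.
; On BeginPlay it binds MoveGate to the boss's enemy-died event.
; MoveGate plays an optional level sequence cutscene, waits a configurable delay, then sets a flag.
; While that flag is set, Tick rotates the left and right GardianAngel components toward their target rotations at constant speed.
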(event `self.ReceiveBeginPlay`
  (bind _bossref (`self.BossRef`))
  ;[1 1 1] Set Up Call Event
  (if (`KismetSystemLibrary.IsValid` _bossref)
    (add `/Game/Blueprints/Enemies/CNS_Enemy_Base_BP.EnemyDied` _bossref (delegate `MoveGate`))))

(event `MoveGate`
  ;[1 1 1] Move the gate
  (`self.Play Cut Scene`)
  (`KismetSystemLibrary.Delay` (`self.DelayBeforeOpenGate`))
  (set `self.ShouldMove` true))

(event `self.ReceiveTick`
  (params (DeltaSeconds :type "Float (single-precision)"))
  ;[1 1 1] Move the gate
  (if (`self.ShouldMove`)
    (`SceneComponent.K2_SetRelativeRotation` (`self.GardianAngelRight`) (`KismetMathLibrary.RInterpTo_Constant` (`SceneComponent.RelativeRotation` (`self.GardianAngelRight`)) (`self.RightRotateTo`) DeltaSeconds (`self.RotateSpeed`)) false false)
    (`SceneComponent.K2_SetRelativeRotation` (`self.GardianAngelLeft`) (`KismetMathLibrary.RInterpTo_Constant` (`SceneComponent.RelativeRotation` (`self.GardianAngelLeft`)) (`self.LeftRotateTo`) DeltaSeconds (`self.RotateSpeed`)) false false)))

(event `Play Cut Scene`
  (bind _levelsequence (`self.LevelSequence`))
  (`/Engine/EditorBlueprintResources/StandardMacros.IsValid` _levelsequence
    (:`Is Valid`
      (bind _outactor (`LevelSequencePlayer.CreateLevelSequencePlayer` _levelsequence))
      (`MovieSceneSequencePlayer.Play` (`LevelSequenceActor.SequencePlayer` _outactor)))))

(fn `UserConstructionScript`)