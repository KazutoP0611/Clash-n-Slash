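; A trigger light object that ignites when hit by the player's fire projectile.
; On BeginPlay it hides its point light and particle system.
; The first sphere hit by a CNS_Projectile_BP sets a one-shot flag, shows both components and calls GotTriggered to notify other logic.
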(event `self.ReceiveBeginPlay`
  ;[1 1 1] Start  Up
  (`SceneComponent.SetVisibility` (`self.PointLight`) false false)
  (`SceneComponent.SetVisibility` (`self.ParticleSystem`) false false))

(event `self.Sphere.OnComponentHit`
  (params (HitComponent :type "PrimitiveComponent Object Reference") (OtherActor :type "Actor Object Reference") (OtherComp :type "PrimitiveComponent Object Reference") (NormalImpulse :type "Vector Structure") (Hit :type "HitResult Structure (by ref)"))
  ;[1 1 1] Get Hit by Player's fire
  (if (not (`self.IsGotTriggered`))
    (cast `/Game/Blueprints/Projectiles/CNS_Projectile_BP` OtherActor)
    (set `self.IsGotTriggered` true)
    (`SceneComponent.SetVisibility` (`self.PointLight`) true false)
    (`SceneComponent.SetVisibility` (`self.ParticleSystem`) true false)
    (`self.GotTriggered`)))

(fn `UserConstructionScript`)