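; Gate actor that opens or shifts its Fences component once the linked triggers have fired.
; Binds to GotTriggered on ArrayOfTrigger and counts calls until the count equals the array length.
; It then plays an optional LevelSequence between configurable delays and starts the move.
; Tick interpolates the fences' relative location toward EndPoint at constant speed, derived from the start-to-end distance over MoveInSeconds.
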(event `PlaySequence`
  (bind _levelsequence (`self.LevelSequence`))
  ;[1 1 1] Play Sequence
  (`/Engine/EditorBlueprintResources/StandardMacros.IsValid` _levelsequence
    (:`Is Valid`
      (bind _outactor (`LevelSequencePlayer.CreateLevelSequencePlayer` _levelsequence))
      (`MovieSceneSequencePlayer.Play` (`LevelSequenceActor.SequencePlayer` _outactor)))))

(event `self.ReceiveBeginPlay`
  ;[1 1 1] Set Up Call Event
  (if (`KismetArrayLibrary.Array_IsValidIndex` (`self.ArrayOfTrigger`))
    (add `/Game/Blueprints/Objects/TriggerFireLight_BP.GotTriggered` (`self.ArrayOfTrigger`) (delegate `CheckTriggered`))))

(event `CheckTriggered`
  ;[1 1 1] Set Up Call Event
  (bind _output_get (set `self.TriggeredCount` (+ 1 (`self.TriggeredCount`))))
  (if (== _output_get (`KismetArrayLibrary.Array_Length` (`self.ArrayOfTrigger`)))
    (`/Engine/EditorBlueprintResources/StandardMacros.IsValid` (`self.LevelSequence`)
      (:`Is Valid`
        (`KismetSystemLibrary.Delay` (`self.DelayBeforePlaySequence`))
        (`self.PlaySequence`)
        (`KismetSystemLibrary.Delay` (`self.DelayAfterPlaySequence`)))
      (:`Is Not Valid`
        _))
    (`self.MoveGate`)))

(event `MoveGate`
  ;[1 1 1] Move the gate
  (set `self.ShouldMove` true))

(event `self.ReceiveTick`
  (params (DeltaSeconds :type "Float (single-precision)"))
  ;[1 1 1] Move the gate
  (if (`self.ShouldMove`)
    (`SceneComponent.K2_SetRelativeLocation` (`self.Fences`) (`KismetMathLibrary.VInterpTo_Constant` (`SceneComponent.RelativeLocation` (`self.Fences`)) (`self.EndPoint`) DeltaSeconds (/ (`KismetMathLibrary.Vector_Distance` (`self.StartPoint`) (`self.EndPoint`)) (`self.MoveInSeconds`))) false false)))

(fn `UserConstructionScript`)